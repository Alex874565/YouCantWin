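; BP_EnemySpawner is an actor that spawns waves of BP_EnemyMelee AI each time SendSpawnSignal is called.
; Each wave adds one enemy, but every fifth resets the count to one and sets Damage to a fixed value, and every tenth also raises Armor.
; A loop spawns the enemies at the spawner's location with a random vertical offset, copying the current Armor and Damage onto each.
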(event `self.ReceiveBeginPlay`)

(event `/Game/Blueprints/BPI_Spawn.SendSpawnSignal`
  (bind _wave (`self.Wave`))
  (bind _counter (`self.Counter`))
  (set `self.Wave` (+ 1 _wave))
  (if (== (mod _wave 5) 0)
    (set `self.EnemyNo` 1)
    (set `self.Damage` 5.0)
    (if (== (mod _wave 10) 0)
      (set `self.Armor` (+ (`self.Armor`) 5.0)))
    (else
      (set `self.EnemyNo` (+ (`self.EnemyNo`) 1))))
  (set `self.Counter` (`self.EnemyNo`))
  (while (> _counter 0)
    (set `self.Counter` (- _counter 1))
    (bind _returnvalue (`AIBlueprintHelperLibrary.SpawnAIFromClass` "/Game/Blueprints/BP_EnemyMelee.BP_EnemyMelee_C" null (+ (`self.K2_GetActorLocation`) (`KismetMathLibrary.MakeVector` 0.0 0.0 (`KismetMathLibrary.RandomFloatInRange` -150.0 200.0))) (struct) false null))
    (bind _asbp_enemy_melee (cast `/Game/Blueprints/BP_EnemyMelee` _returnvalue))
    (set `/Game/Blueprints/BP_EnemyMelee.Armor` (`self.Armor`) _asbp_enemy_melee)
    (set `/Game/Blueprints/BP_EnemyMelee.Damage` (`self.Damage`) _asbp_enemy_melee)))

(fn `UserConstructionScript`)