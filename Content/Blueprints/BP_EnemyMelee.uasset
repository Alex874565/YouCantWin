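; Paper2D melee enemy character that attacks targets in front of it, takes armor-reduced hits and is destroyed at zero health.
; Tick sphere-traces along the sprite's facing, plays the attack flipbook, then re-traces after a windup delay before sending damage to the target.
; Hits knock it away from the player along X.
; LinkReachable launches it toward nav link destinations using velocity computed by math expressions.
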(event EventBeginPlay
  (Development|PrintString (Utilities|String|ToString(Float) (Variables|Default|GetArmor)))
  (Development|PrintString (Utilities|String|ToString(Float) (Variables|Default|GetDamage))))

(event EventLinkReachable
  (params (NavLinkProxiDestination :type Vector :default "0, 0, 0"))
  (bind (_x _y _z) (Math|Vector|BreakVector NavLinkProxiDestination))
  (bind _returnvalue (Transformation|GetActorLocation))
  (bind (_x_2 _y_2 _z_2) (Math|Vector|BreakVector _returnvalue))
  (Character|LaunchCharacter (Math|Vector|MakeVector (|((DestinationX-StartX)/{42BB3699-4E92-5CEA-E0FF-DFBDB3D80F21}) _x _x_2) (|((DestinationY-StartY)/{42BB3699-4E92-5CEA-E0FF-DFBDB3D80F21}) _y _y_2) (|((DestinationHeight-(StartHeight-(((Power({42BB3699-4E92-5CEA-E0FF-DFBDB3D80F21},2))*0.500000)*{3BF7127D-4785-97A1-D484-E38C6E80AE22})))/{42BB3699-4E92-5CEA-E0FF-DFBDB3D80F21}) _z _z_2)) true true))

(event EventHit
  (params (Damage :type Float%20%28double-precision%29))
  (Variables|Default|SetHealth (- (Variables|Default|GetHealth) (- Damage (Variables|Default|GetArmor))))
  (if (< (.x (Transformation|GetActorLocation (Game|GetPlayerCharacter 0))) (.x (Transformation|GetActorLocation)))
    (Character|LaunchCharacter "600.000000,0.000000,0.000000" false false)
    (else
      (Character|LaunchCharacter "-600.000000,0.000000,0.000000" false false))))

(event EventTick
  (params (DeltaSeconds :type Float%20%28single-precision%29))
  (bind _returnvalue (Transformation|GetActorLocation))
  (bind _returnvalue_2 (Transformation|GetActorLocation))
  (if (<= (Variables|Default|GetHealth) 0.0)
    (Actor|DestroyActor)
    (else
      (bind _returnvalue_3 (Collision|SphereTraceByChannel _returnvalue_2 (+ _returnvalue_2 (* (Math|Rotator|GetRotationXVector (Transformation|GetWorldRotation (Variables|Default|GetSprite))) (Variables|Default|GetAttackDist))) 5.0 "TraceTypeQuery3" false 0 "None"))
      (if (and _returnvalue_3 (not (Variables|Default|GetisAttacking)))
        (Variables|Default|SetisAttacking true)
        (Sprite|SetFlipbook (Variables|Default|GetSprite) "/Game/Assets/Flipbooks/FB_EnemyMeleeAttack.FB_EnemyMeleeAttack")
        (Utilities|FlowControl|Delay 0.4)
        (bind (_outhit _returnvalue_4) (Collision|SphereTraceByChannel _returnvalue (+ _returnvalue (* (Math|Rotator|GetRotationXVector (Transformation|GetWorldRotation (Variables|Default|GetSprite))) (Variables|Default|GetAttackDist))) 5.0 "TraceTypeQuery3" false 0 "None"))
        (if _returnvalue_4
          (Class|BPIHit|Hit(Message) (.HitActor (Collision|BreakHitResult _outhit)) (Variables|Default|GetDamage))
          (Utilities|FlowControl|Delay 0.2))
        (Sprite|SetFlipbook (Variables|Default|GetSprite) "/Game/Assets/Flipbooks/FB_EnemyMeleeWalk.FB_EnemyMeleeWalk")
        (Variables|Default|SetisAttacking false)))))

(fn ConstructionScript)