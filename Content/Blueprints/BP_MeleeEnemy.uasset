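; Melee enemy character Blueprint whose only active logic is jumping across nav links.
; LinkReachable_1 receives a link destination and calls LaunchCharacter from the actor's location, overriding XY and Z velocity.
; Math Expression nodes derive ballistic launch velocity per axis, dividing offsets by JumpDistance and adding a gravity term on Z.
; JumpDistance is zero for X and Y, and the Z node's gravity, power base and JumpDistance inputs are not supplied.
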(event Custom|LinkReachable_1
  (params (NavLinkProxiDestination :type Vector))
  (bind (_x _y _z) (Math|Vector|BreakVector NavLinkProxiDestination))
  (bind _returnvalue (Transformation|GetActorLocation))
  (bind (_x_2 _y_2 _z_2) (Math|Vector|BreakVector _returnvalue))
  (Character|LaunchCharacter (Math|Vector|MakeVector (|((DestinationX-StartX)/JumpDistance) _x _x_2 0.0) (|((DestinationY-StartY)/JumpDistance) _y _y_2 0.0) (|((DestinationHeight-(StartHeight-(((Power(None,2))*0.500000)*Gravity)))/JumpDistance) _z _z_2 0.0 0.0 0.0)) true true))

(event EventBeginPlay)

(event Collision|EventActorBeginOverlap
  (params (OtherActor :type Actor%20Object%20Reference)))

(fn ConstructionScript)