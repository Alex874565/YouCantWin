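; BP_Player is a player character with flipbook animation that moves back and forth along a single axis.
; On BeginPlay it casts its controller to BP_PlayerController and registers the IMC_Default Enhanced Input mapping context.
; IA_Movement feeds its signed value into movement along the actor's forward vector, plays the run flipbook and flips the sprite's world rotation to face the direction of travel.
; When the input completes, the sprite returns to the idle flipbook.
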(event `self.ReceiveBeginPlay`
  (bind _asbp_player_controller (cast `/Game/Blueprints/BP_PlayerController` (`self.GetController`)))
  (`EnhancedInputSubsystemInterface.AddMappingContext` (pcsubsystem `EnhancedInputLocalPlayerSubsystem` _asbp_player_controller) "/Game/Blueprints/IMC_Default.IMC_Default" 0 (struct)))

(event `EnhancedInput|/Game/Blueprints/IA_Movement`
  (params (ActionValue :type "Float (double-precision)") (ElapsedSeconds :type "Float (double-precision)") (TriggeredSeconds :type "Float (double-precision)") (InputAction :type "InputAction Object Reference" :default "/Game/Blueprints/IA_Movement.IA_Movement"))
  (:`Triggered`
    (`self.AddMovementInput` (`self.GetActorForwardVector`) ActionValue)
    (`PaperFlipbookComponent.SetFlipbook` (`self.Sprite`) "/Game/Assets/Flipbooks/FB_Run.FB_Run")
    (if (> ActionValue 0.0)
      (`SceneComponent.K2_SetWorldRotation` (`self.Sprite`) (struct) false false)
      (else
        (`SceneComponent.K2_SetWorldRotation` (`self.Sprite`) (struct :`Yaw` -180.0) false false))))
  (:`Completed`
    (`PaperFlipbookComponent.SetFlipbook` (`self.Sprite`) "/Game/Assets/Flipbooks/FB_Idle.FB_Idle")))

(fn `UserConstructionScript`)